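; BP_MoveActor is a pawn that wanders endlessly between random points inside configurable X/Y bounds.
; On BeginPlay it applies Speed to its FloatingPawnMovement, then uses AI MoveTo toward a random target at its current height.
; Success, failure or a hit on its Cube component calls MoveToTarget again to pick a new destination.
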(event `self.ReceiveBeginPlay`
  ;[1 1 1] Set max speed and start move
  (set `FloatingPawnMovement.MaxSpeed` (`self.Speed`) (`self.FloatingPawnMovement`))
  (`self.MoveToTarget`))

(event `MoveToTarget`
  ;[1 1 1] Move actor
  (bind _result (`self.NewRandomTarget`))
  (`|AIMoveTo` (`self.FloatingPawnMovement`) self _result null
    (:`OnSuccess`
      _)
    (:`OnFail`
      _))
  (`self.MoveToTarget`))

(event `self.Cube.OnComponentHit`
  (params (HitComponent :type "PrimitiveComponent Object Reference") (OtherActor :type "Actor Object Reference") (OtherComp :type "PrimitiveComponent Object Reference") (NormalImpulse :type "Vector Structure") (Hit :type "HitResult Structure (by ref)"))
  (`self.MoveToTarget`))

(fn `NewRandomTarget`
  (returns (Result :type "Vector Structure"))
  (bind (_returnvalue_x _returnvalue_y _returnvalue_z) (`KismetMathLibrary.BreakVector` (`self.K2_GetActorLocation`)))
  ;[1 1 1] Get new target location
  (return (`KismetMathLibrary.MakeVector` (`KismetMathLibrary.RandomFloatInRange` (`self.MinX`) (`self.MaxX`)) (`KismetMathLibrary.RandomFloatInRange` (`self.MinY`) (`self.MaxY`)) _returnvalue_z)))

(fn `UserConstructionScript`)